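; Floating scene object that offsets its mesh vertically, starting on BeginPlay.
; A timeline's alpha lerps FloatingMesh's relative location from zero to FloatDistance on Z.
; StartFloating and StopFloating events play and stop the timeline.
; The construction script passes PlaybackRate to SetNewTime, which sets the timeline's position rather than its play rate.
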(event `self.ReceiveBeginPlay`
  (`self.StartFloating`))

(event `StartFloating`
  (bind (_direction _alpha) (`Timeline|FloatingTimeline` :!label _label)
    (:`Update`
      (`SceneComponent.K2_SetRelativeLocation` (`self.FloatingMesh`) (`KismetMathLibrary.VLerp` (0.0 0.0 0.0) (`KismetMathLibrary.MakeVector` 0.0 0.0 (`self.FloatDistance`)) _alpha) false false))))

(event `StopFloating`
  (goto _label :!via `Stop`))

(fn `UserConstructionScript`
  (`TimelineComponent.SetNewTime` (`self.FloatingTimeline`) (`self.PlaybackRate`)))