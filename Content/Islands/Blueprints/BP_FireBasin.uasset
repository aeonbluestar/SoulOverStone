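; BP_FireBasin is a placeable stone fire basin prop with an optional fire effect and light.
; All setup runs in the construction script, with no active event graph logic.
; A custom materials flag swaps the stone and statue materials on the mesh.
; A fire flag toggles the fire and light visibility, then applies exposed light intensity, color, shadow and radius, or zeroes intensity when off.
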(fn `UserConstructionScript`
  (bind _use_custom_materials (`self.Use Custom Materials`))
  (bind _is_it_fire_ (`self.Is it Fire?`))
  (`|ExecutionSequence`
    (:`then_0`
      (if _use_custom_materials
        ;[1 1 1] Set Stone Material
        (`PrimitiveComponent.SetMaterial` (`self.FireBasin`) 1 (`self.Stone Material`))))
    (:`then_1`
      (if _use_custom_materials
        ;[1 1 1] Set Statue Material
        (`PrimitiveComponent.SetMaterial` (`self.FireBasin`) 0 (`self.Statue Material`))))
    (:`then_2`
      ;[1 1 1] Toggle Fire
      (`SceneComponent.SetVisibility` (`self.P_StoneBasinFire`) _is_it_fire_ false)
      (`SceneComponent.SetVisibility` (`self.FireLight`) _is_it_fire_ false)
      (if _is_it_fire_
        ;[1 1 1] Set Fire Light Intensity
        (`LightComponent.SetIntensity` (`self.FireLight`) (`self.Light Intensity`))
        ;[1 1 1] Set Fire Light Color
        (`LightComponent.SetLightColor` (`self.FireLight`) (`self.Light Color`) true)
        ;[1 1 1] Toggle Fire Light Cast Shadow
        (`LightComponentBase.SetCastShadows` (`self.FireLight`) (`self.Cast Shadow`))
        ;[1 1 1] Set Fire Light Attenuation Radius
        (`LocalLightComponent.SetAttenuationRadius` (`self.FireLight`) (`self.Attenuation Radius`))
        (else
          (`LightComponent.SetIntensity` (`self.FireLight`) 0.0))))))