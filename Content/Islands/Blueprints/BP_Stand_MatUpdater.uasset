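; Configurable stand actor that swaps its static mesh and restyles its material from exposed variables, entirely in the Construction Script.
; It creates a dynamic instance of Material0 on slot 0, then pushes glow, metalness toggle, optional roughness and UV scale through mesh-wide parameter setters.
; Texture overrides go to that instance, with base color, tint noise, normal and ORME each behind a toggle and the emissive noise mask always applied.
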(fn `UserConstructionScript`
  (locals (NewLocalVar_0 :type "Texture Object Reference"))
  ;[1 1 1] Update Mesh
  (`StaticMeshComponent.SetStaticMesh` (`self.Mesh`) (`self.Change Mesh`))
  ;[1 1 1 1 35] Material 0
  ;;[1 1 1] Set Up Dynamic Material
  (bind _returnvalue (`KismetMaterialLibrary.CreateDynamicMaterialInstance` (`self.Material 0`)))
  (`|ExecutionSequence`
    (:`then_0`
      (bind _output_get (set `self.My Dynamic Material` _returnvalue))
      (`PrimitiveComponent.SetMaterial` (`self.Mesh`) 0 _output_get)
      (`|ExecutionSequence`
        (:`then_0`
          ;;[1 1 1] Emissive
          (`MeshComponent.SetScalarParameterValueOnMaterials` (`self.Mesh`) "Glow Intensity" (`self.Glow Intensity`))
          (`MeshComponent.SetVectorParameterValueOnMaterials` (`self.Mesh`) "Glow Color" (`KismetMathLibrary.Conv_LinearColorToVector` (`self.Glow Color`)))
          (`MeshComponent.SetScalarParameterValueOnMaterials` (`self.Mesh`) "Emissive Noise UV Scale" (`self.Emissive Noise Scale`)))
        (:`then_1`
          ;;[1 1 1] Metallic
          (if (`self.Is It Metal?`)
            (`MeshComponent.SetScalarParameterValueOnMaterials` (`self.Mesh`) "Metalness Value" 1.0)
            (else
              (`MeshComponent.SetScalarParameterValueOnMaterials` (`self.Mesh`) "Metalness Value" 0.0))))
        (:`then_2`
          ;;[1 1 1] Roughness
          (if (`self.Adjust Roughness?`)
            (`MeshComponent.SetScalarParameterValueOnMaterials` (`self.Mesh`) "Roughness Value" (`self.Roughness`))))
        (:`then_3`
          ;;[1 1 1] UV Scaling
          (`MeshComponent.SetScalarParameterValueOnMaterials` (`self.Mesh`) "UV Scale" (`self.UV Scale`)))))
    (:`then_1`
      ;;[1 1 1] Base Color Textures
      (if (`self.Update Base Color`)
        (`MaterialInstanceDynamic.SetTextureParameterValue` _output_get "Base Color Texture" (`self.Base Color`))))
    (:`then_2`
      (if (`self.Update Tint Noise`)
        (`MaterialInstanceDynamic.SetTextureParameterValue` _output_get "Tint Noise" (`self.Tint Noise`))))
    (:`then_3`
      ;;[1 1 1] Normal Textures
      (if (`self.Update Normal`)
        (`MaterialInstanceDynamic.SetTextureParameterValue` _output_get "Normal Texture" (`self.Normal Map`))))
    (:`then_4`
      ;;[1 1 1] ORME Textures
      (if (`self.Update ORME`)
        (`MaterialInstanceDynamic.SetTextureParameterValue` _output_get "ORME Texture" (`self.ORME`))))
    (:`then_5`
      ;;[1 1 1] Emissive Noise Mask
      (`MaterialInstanceDynamic.SetTextureParameterValue` _output_get "Emissive Noise Mask" (`self.Emissive Noise Mask`)))))